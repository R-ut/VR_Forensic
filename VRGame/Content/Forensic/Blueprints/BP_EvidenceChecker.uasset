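; BP_EvidenceChecker is a Blueprint that scores evidence the player picks in a forensic game.
; Its CheckEvidenceType event takes a target actor and tests its tags for weapon, then explosive evidence.
; A match adds a type-specific amount to a Score variable, with explosives worth more, and prints a pickup message; otherwise it prints that nothing was picked.
; It only evaluates the actor passed in, leaving that actor untouched.
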(event `CheckEvidenceType`
  (params (TargetActor :type "Actor Object Reference"))
  (if (`self.ActorHasTag` TargetActor "Evidence_Weapon")
    (set `self.Score` (+ (`self.Score`) 10))
    (`KismetSystemLibrary.PrintString` "Evidence picked")
    (elif (`self.ActorHasTag` TargetActor "Evidence_Explosive")
      (set `self.Score` (+ (`self.Score`) 15))
      (`KismetSystemLibrary.PrintString` "Evidence picked")
      (else
        (`KismetSystemLibrary.PrintString` "No evidence Picked")))))

(fn `UserConstructionScript`)